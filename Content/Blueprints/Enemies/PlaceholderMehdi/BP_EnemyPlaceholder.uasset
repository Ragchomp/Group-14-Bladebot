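; BP_EnemyPlaceholder is a placeholder enemy that feeds perceived player locations to its AI blackboard.
; The construction script records its spawn location as StartPosition.
; When AI perception senses a Player-tagged actor, it writes the stimulus location to the TargetPosition key.
; Any unsuccessful sense update, regardless of the actor's tag, resets TargetPosition to StartPosition.
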(event OnTargetPerceptionInfoUpdated(AIPerception)
  (params (UpdateInfo :type Actor%20Perception%20Update%20Info%20Structure%20%28by%20ref%29))
  (bind (_targetid _target _stimulus) (Utilities|Struct|BreakActorPerceptionUpdateInfo UpdateInfo))
  (bind (_age _expirationage _strength _stimuluslocation _receiverlocation _tag _bsuccessfullysensed) (Utilities|Struct|BreakAIStimulus _stimulus))
  (if _bsuccessfullysensed
    (if (Actor|ActorHasTag _target "Player")
      (AI|Components|Blackboard|SetValueasVector (AI|GetBlackboard 0) (Utilities|Name|MakeLiteralName "TargetPosition") _stimuluslocation))
    (else
      (AI|Components|Blackboard|SetValueasVector (AI|GetBlackboard 0) (Utilities|Name|MakeLiteralName "TargetPosition") (Variables|Default|GetStartPosition)))))

(event OnTargetPerceptionUpdated(AIPerception)
  (params (Actor :type Actor%20Object%20Reference) (Stimulus :type AI%20Stimulus%20Structure)))

(event EventBeginPlay)

(event Collision|EventActorBeginOverlap
  (params (OtherActor :type Actor%20Object%20Reference)))

(event EventTick
  (params (DeltaSeconds :type Float%20%28single-precision%29)))

(fn ConstructionScript
  (Utilities|FlowControl|Sequence
    (:then_0
      (Variables|Default|SetStartPosition (Transformation|GetActorLocation)))))