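; BP_PlayerDebugDisplay is a debug actor in the Vegard map that shows the player's speed as floating text.
; Each tick it casts the player pawn to BP_bladebot and converts its velocity to meters per second.
; It keeps a smoothed average by blending toward the current speed, scaled by delta time.
; Both values are drawn as a debug string attached to the bladebot.
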(event EventBeginPlay)

(event Collision|EventActorBeginOverlap
  (params (OtherActor :type Actor%20Object%20Reference)))

(event EventTick
  (params (DeltaSeconds :type Float%20%28single-precision%29))
  (bind _asbp_bladebot (Utilities|Casting|CastToBP_bladebot (Game|Player|GetPlayerPawn 0)))
  (Rendering|Debug|DrawDebugString "0, 0, 0" (Utilities|String|ToString(Text) (Utilities|Text|FormatText "Speed {Speed}m/s 
Average {Average}m/s" (/ (Math|Vector|VectorLength (Transformation|GetVelocity _asbp_bladebot)) 1e+02) (+ (* (- (/ (Math|Vector|VectorLength (Transformation|GetVelocity _asbp_bladebot)) 1e+02) (Variables|Default|GetAverage)) DeltaSeconds) (Variables|Default|GetAverage)))) _asbp_bladebot "(R=1.000000,G=1.000000,B=1.000000,A=1.000000)")
  (Variables|Default|SetAverage (+ (* (- (/ (Math|Vector|VectorLength (Transformation|GetVelocity _asbp_bladebot)) 1e+02) (Variables|Default|GetAverage)) DeltaSeconds) (Variables|Default|GetAverage))))

(fn ConstructionScript)