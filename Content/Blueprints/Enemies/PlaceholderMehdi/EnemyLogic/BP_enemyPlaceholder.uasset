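; Placeholder enemy Blueprint that links an enemy actor to its AI Blackboard.
; On BeginPlay it saves its location, writes it to the StartingPoint key, and caches the player as a BP_bladebot.
; UpdateTarget and UpdateSight write the Target and HasLineOfSight keys.
; DamageResponse prints health for debugging, Death only sets a Dead flag, and TriggerAttack is an empty stub.
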(event Custom|DamageResponse
  (params (Health :type Float%20%28double-precision%29))
  (Development|PrintString (Utilities|String|ToString(Float) Health) true true "(R=1.000000,G=0.985763,B=0.000000,A=1.000000)" 2.0 "8"))

(event Custom|Death
  (Variables|Default|SetDead true))

(event EventBeginPlay
  ;[1 1 1] Initialize
  (Utilities|FlowControl|Sequence
    (:then_0
      (Variables|Default|SetStartPosition (Transformation|GetActorLocation)))
    (:then_1
      (AI|Components|Blackboard|SetValueasVector (AI|GetBlackboard 0) (Utilities|Name|MakeLiteralName "StartingPoint") (Variables|Default|GetStartPosition)))
    (:then_2
      (bind _asbp_bladebot (Utilities|Casting|CastToBP_bladebot (Game|GetPlayerCharacter 0)))
      (Variables|Default|SetPlayer _asbp_bladebot))))

(event Collision|EventActorBeginOverlap
  (params (OtherActor :type Actor%20Object%20Reference)))

(event EventTriggerAttack
  (params (Trace :type Hit%20Result%20Structure) (ShotCount :type Integer)))

(fn ConstructionScript)

(fn UpdateTarget
  (params (Target :type Actor%20Object%20Reference))
  (AI|Components|Blackboard|SetValueasObject (AI|GetBlackboard 0) (Utilities|Name|MakeLiteralName "Target") Target))

(fn UpdateSight
  (params (Has%20Line%20Of%20Sight :type Boolean))
  (AI|Components|Blackboard|SetValueasBool (AI|GetBlackboard 0) (Utilities|Name|MakeLiteralName "HasLineOfSight") Has%20Line%20Of%20Sight))