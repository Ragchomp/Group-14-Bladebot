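; Grappling hook projectile for the bladebot player, fired along the camera's forward direction with a cable attached to the player's mesh socket.
; A visibility trace sets cable length and direction, then a physics impulse launches the box, and the actor destroys itself if nothing is hit in time.
; On impact it freezes, records the hit and notifies the player.
; After a short grace period, its sphere stops reeling and clears the hook when the player overlaps it.
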(event OnComponentHit(Box)
  (params (HitComponent :type Primitive%20Component%20Object%20Reference) (OtherActor :type Actor%20Object%20Reference) (OtherComp :type Primitive%20Component%20Object%20Reference) (NormalImpulse :type Vector :default "0, 0, 0") (Hit :type Hit%20Result%20Structure%20%28by%20ref%29))
  ;[1 1 1] Hook Hit
  (Utilities|FlowControl|Sequence
    (:then_0
      (Variables|TraceResults|SetHit true))
    (:then_1
      (Physics|SetSimulatePhysics (Variables|Default|GetBox) false))
    (:then_2
      (Default|HookHit (Variables|Components|GetPlayerCharacter)))
    (:then_3
      (bind _returnvalue (AddComponent|AddSceneComponent false (Math|Transform|MakeTransform (stale _output_get_2) "0, 0, 0" "1.000000,1.000000,1.000000")))
      (bind _output_get (Variables|Default|SetHookTarget _returnvalue))
      (Transformation|SetWorldRotation _output_get "0, 0, 0" false false))
    (:then_4
      (bind _output_get_2 (Variables|TraceResults|SetHit%20Location (.location Hit))))
    (:then_5
      (Variables|TraceResults|SetHitOrientationVector (.normal Hit)))
    (:then_6
      (Transformation|SetWorldTransform (Variables|Default|GetCone) (Transformation|GetWorldTransform (Variables|Default|GetHookTarget)) false false))))

(event OnComponentBeginOverlap(Sphere)
  (params (OverlappedComponent :type Primitive%20Component%20Object%20Reference) (OtherActor :type Actor%20Object%20Reference) (OtherComp :type Primitive%20Component%20Object%20Reference) (OtherBodyIndex :type Integer) (bFromSweep :type Boolean) (SweepResult :type Hit%20Result%20Structure%20%28by%20ref%29))
  ;[1 1 1] Kill In sphere
  (bind _asbp_bladebot (Utilities|Casting|CastToBP_bladebot OtherActor))
  (Default|StopReel (Variables|/Game/Blueprints/Character/BP_bladebot.BP_bladebot_C|GetMovementController (Variables|Components|GetPlayerCharacter)))
  (Default|Clearhook _asbp_bladebot))

(event EventBeginPlay
  (bind _sphere (Variables|Default|GetSphere))
  (bind _box (Variables|Default|GetBox))
  (Utilities|FlowControl|Sequence
    (:then_0
      ;[1 1 1] Setup
      (bind _asbp_bladebot (Utilities|Casting|CastToBP_bladebot (Game|Player|GetPlayerPawn 0)))
      (Variables|Components|SetPlayerCharacter _asbp_bladebot))
    (:then_1
      (Class|CableComponent|SetAttachEndto (Variables|Default|GetHookCable) (Variables|Components|GetPlayerCharacter) "Mesh" "GrapplingHookSlot"))
    (:then_2
      ;[1 1 1] Calculate direction
      (bind _outhit (Collision|LineTraceByChannel (Transformation|GetActorLocation (Variables|Components|GetPlayerCharacter)) (+ (Transformation|GetActorLocation (Variables|Components|GetPlayerCharacter)) (* (Math|Vector|GetForwardVector (Variables|/Game/Blueprints/Character/BP_bladebot.BP_bladebot_C|GetCamera (Variables|Components|GetPlayerCharacter))) (Variables|HookVariable|GetHookDirMultiplier))) "TraceTypeQuery1" false 0 "None"))
      (Variables|HookVariable|SetCableLength (.Distance (Collision|BreakHitResult _outhit)))
      (Variables|HookVariable|SetHookDirection (Math|Vector|GetUnitDirection(Vector) (.TraceStart (Collision|BreakHitResult _outhit)) (.TraceEnd (Collision|BreakHitResult _outhit)))))
    (:then_3
      ;[1 1 1] Fire Hook
      (Physics|SetSimulatePhysics _box true)
      (Physics|AddImpulse _box (* (Variables|HookVariable|GetHookDirection) (Variables|HookVariable|GetHookSpeed)) "None" true))
    (:then_4
      ;[1 1 1] Destroy If Miss
      (Utilities|FlowControl|Delay (Variables|HookVariable|GetHookRange))
      (if (not (Variables|TraceResults|GetHit))
        (Actor|DestroyActor)))
    (:then_5
      ;[1 1 1] Grace Period KillSphere
      (Variables|/Script/Engine.PrimitiveComponent|SetbGenerateOverlapEvents _sphere false)
      (Utilities|FlowControl|Delay 0.5)
      (Variables|/Script/Engine.PrimitiveComponent|SetbGenerateOverlapEvents _sphere true))))

(fn ConstructionScript)