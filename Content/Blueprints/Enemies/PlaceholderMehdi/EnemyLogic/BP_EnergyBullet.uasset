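; BP_EnergyBullet is an enemy homing projectile that seeks the BP_bladebot actor and damages anything tagged Player that overlaps its sphere.
; After a short delay, Tick eases its homing acceleration and velocity down to zero.
; Coming to a stop or hitting the player triggers destruction, which ramps a Niagara DestructionFloat parameter before destroying the actor.
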(event OnComponentBeginOverlap(Sphere)
  (params (OverlappedComponent :type Primitive%20Component%20Object%20Reference) (OtherActor :type Actor%20Object%20Reference) (OtherComp :type Primitive%20Component%20Object%20Reference) (OtherBodyIndex :type Integer) (bFromSweep :type Boolean) (SweepResult :type Hit%20Result%20Structure%20%28by%20ref%29))
  (if (Actor|ActorHasTag OtherActor "Player")
    (Class|BPIDamage|Damage(Message) OtherActor true 25.0 1.0 "NewEnumerator0" "NewEnumerator0")
    (Variables|Default|SetDestruction true)))

(event EventBeginPlay
  (Utilities|FlowControl|Sequence
    (:then_0
      (bind _returnvalue (Actor|GetActorOfClass "/Game/Blueprints/Character/BP_bladebot.BP_bladebot_C"))
      (Variables|/Script/Engine.ProjectileMovementComponent|SetHomingTargetComponent (Variables|Default|GetProjectileMovement) (Variables|/Script/Engine.Actor|GetRootComponent _returnvalue)))
    (:then_1
      (Utilities|FlowControl|Delay 2.0)
      (Variables|Default|SetDeceleration true))))

(event EventTick
  (params (DeltaSeconds :type Float%20%28single-precision%29))
  (if (Variables|Default|GetDestruction)
    (Utilities|FlowControl|Sequence
      (:then_0
        (Variables|Default|SetNiagaraDestructionFloat (Math|Interpolation|FInterpTo (Variables|Default|GetNiagaraDestructionFloat) 1.0 DeltaSeconds 6.0)))
      (:then_1
        (Niagara|SetNiagaraVariable(Float) (Variables|Default|GetEnemyProjectile) "DestructionFloat" (Variables|Default|GetNiagaraDestructionFloat)))
      (:then_2
        (if (== (Variables|Default|GetNiagaraDestructionFloat) 1.0)
          (Actor|DestroyActor))))
    (elif (Variables|Default|GetDeceleration)
      (Utilities|FlowControl|Sequence
        (:then_0
          (Variables|/Script/Engine.ProjectileMovementComponent|SetHomingAccelerationMagnitude (Variables|Default|GetProjectileMovement) (Math|Interpolation|FInterpTo (Variables|/Script/Engine.ProjectileMovementComponent|GetHomingAccelerationMagnitude (Variables|Default|GetProjectileMovement)) 0.0 DeltaSeconds 2.0)))
        (:then_1
          (bind _output_get (Variables|/Script/Engine.MovementComponent|SetVelocity (Variables|Default|GetProjectileMovement) (Math|Interpolation|VInterpTo (Variables|/Script/Engine.MovementComponent|GetVelocity (Variables|Default|GetProjectileMovement)) "0, 0, 0" DeltaSeconds 3.0)))
          (if (Utilities|Operators|EqualEqual :A _output_get)
            (Variables|Default|SetDestruction true)))))))

(fn ConstructionScript)