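; BP_Constraint is the physics tether between the player's grappling hook and the bladebot's physics body.
; On BeginPlay it finds the player's movement controller, hook reference and physics parent, then constrains the hook's cone to the physics cube.
; All three linear axes are limited to twice the hook's cable length, so the constraint acts like a rope.
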(event EventBeginPlay
  (bind _physicsconstraint (Variables|Default|GetPhysicsConstraint))
  (Utilities|FlowControl|Sequence
    (:then_0
      ;[1 1 1] Initialize
      (Utilities|FlowControl|Sequence
        (:then_0
          (bind _asbp_bladebot (Utilities|Casting|CastToBP_bladebot (Game|GetPlayerCharacter 0)))
          (Variables|Default|SetPlayer _asbp_bladebot))
        (:then_1
          (Variables|Default|SetMovement (Variables|/Game/Blueprints/Character/BP_bladebot.BP_bladebot_C|GetMovementController (Variables|Default|GetPlayer))))
        (:then_2
          (Variables|Default|SetPhysicsTarget (Variables|/Game/Blueprints/Character/BP_bladebot.BP_bladebot_C|GetPhysicsParent (Variables|Default|GetPlayer))))
        (:then_3
          (Variables|Default|SetHook (Variables|/Game/Blueprints/Character/BP_BladebotMovementController.BP_BladebotMovementController_C|GetHookRef (Variables|Default|GetMovement))))))
    (:then_1
      ;[1 1 1] Attach and set up Constraint
      (Utilities|FlowControl|Sequence
        (:then_0
          (Class|PhysicsConstraintComponent|SetConstrainedComponents (Variables|Default|GetPhysicsConstraint) (Variables|/Game/Blueprints/Objects/Hook/BP_GrapplingHook.BP_GrapplingHook_C|GetCone (Variables|Default|GetHook)) "None" (Variables|/Game/Blueprints/Objects/Hook/BP_PhysicsAttachment.BP_PhysicsAttachment_C|GetPhysicscube (Variables|Default|GetPhysicsTarget)) "None"))
        (:then_1
          (Class|PhysicsConstraintComponent|SetLinearXLimit _physicsconstraint "LCM_Limited" (* (Variables|/Game/Blueprints/Objects/Hook/BP_GrapplingHook.BP_GrapplingHook_C|GetCableLength (Variables|Default|GetHook)) 2.0))
          (Class|PhysicsConstraintComponent|SetLinearYLimit _physicsconstraint "LCM_Limited" (* (Variables|/Game/Blueprints/Objects/Hook/BP_GrapplingHook.BP_GrapplingHook_C|GetCableLength (Variables|Default|GetHook)) 2.0))
          (Class|PhysicsConstraintComponent|SetLinearZLimit _physicsconstraint "LCM_Limited" (* (Variables|/Game/Blueprints/Objects/Hook/BP_GrapplingHook.BP_GrapplingHook_C|GetCableLength (Variables|Default|GetHook)) 2.0)))))))

(fn ConstructionScript)