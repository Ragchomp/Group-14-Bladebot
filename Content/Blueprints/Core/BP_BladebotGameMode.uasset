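; Game mode for Bladebot that restores level enemies and objectives when the player restarts.
; Shortly after BeginPlay it caches mine enemies with patrol targets, objective points and ship objectives, plus their transforms.
; OnRestartPlayer triggers a delayed, DoOnce-guarded reset that respawns them from the cached data and clears the player's GameComplete flag.
; Enemies and objective points are destroyed first, but the ship loop's DestroyActor targets the game mode itself.
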(event EventBeginPlay
  (Utilities|FlowControl|Sequence
    (:then_0
      ;[1 1 1] Saves all ship objective point
      (Utilities|FlowControl|Sequence
        (:then_0
          (Utilities|FlowControl|Delay 0.1)
          (bind _outactors (Actor|GetAllActorsOfClass "/Game/Blueprints/Objectives/BP_UpdatedShipObjective.BP_UpdatedShipObjective_C"))
          (bind _output_get (Variables|Default|SetShipObjectives _outactors))
          (for _array_element _output_get
            (Utilities|Array|Insert (Variables|Default|GetShipObjectiveTransforms) (Transformation|GetActorTransform _array_element))))))
    (:then_1
      ;[1 1 1] Saves all objective point
      (Utilities|FlowControl|Sequence
        (:then_0
          (Utilities|FlowControl|Delay 0.1)
          (bind _outactors_2 (Actor|GetAllActorsOfClass "/Game/Blueprints/Objectives/BP_UpdatedObjectivePoint.BP_UpdatedObjectivePoint_C"))
          (bind _output_get_2 (Variables|Default|SetLevelObjectives _outactors_2))
          (for (_array_element_2 _array_index) _output_get_2
            (Utilities|Array|Insert (Variables|Default|GetObjectiveTransforms) (Transformation|GetActorTransform _array_element_2) _array_index)))))
    (:then_2
      ;[1 1 1] Saves all Enemy info
      (Utilities|FlowControl|Sequence
        (:then_0
          (Utilities|FlowControl|Delay 0.1)
          (bind _outactors_3 (Actor|GetAllActorsOfClass "/Game/Blueprints/Enemies/BP_MineEnemy.BP_MineEnemy_C"))
          (bind _output_get_3 (Variables|Default|SetLevelEnemis _outactors_3))
          (for (_array_element_3 _array_index_2) _output_get_3
            (Utilities|Array|Insert (Variables|Default|GetAll%20Enmy%20details) (Utilities|Struct|MakeBPS_EnemyStruct (Transformation|GetActorTransform _array_element_3) (Variables|/Script/BladeBot.MineEnemy|GetPatrolTargets _array_element_3)) _array_index_2)))))))

(event EventOnRestartPlayer
  (params (NewPlayer :type Controller%20Object%20Reference))
  (Utilities|FlowControl|Sequence
    (:then_0
      (Utilities|FlowControl|Delay 0.5)
      (goto _label Reset))
    (:then_1
      (Utilities|FlowControl|DoOnce true :!label _label
        (:Completed
          (Utilities|FlowControl|Delay 0.2)
          (CallFunction|ResetObjectives&Enemies))))))

(fn ConstructionScript)

(fn ResetObjectives&Enemies
  (Utilities|FlowControl|Sequence
    (:then_0
      ;[1 1 1] Resets enemies
      (Utilities|FlowControl|DoOnce false :!label _label
        (:Completed
          (bind _outactors (Actor|GetAllActorsOfClass "/Game/Blueprints/Enemies/BP_MineEnemy.BP_MineEnemy_C"))
          (for _array_element _outactors
            (Actor|DestroyActor _array_element))
          (for (_array_element_2 _array_index) (Variables|Default|GetLevelEnemis)
            (bind _returnvalue (Game|SpawnActorfromClass (Utilities|GetClass _array_element_2) (.transform (Utilities|Array|Get(acopy) (Variables|Default|GetAll%20Enmy%20details) _array_index)) "Undefined" "MultiplyWithRoot" 0 0))
            (Variables|/Script/BladeBot.MineEnemy|SetPatrolTargets _returnvalue (.targets (Utilities|Array|Get(acopy) (Variables|Default|GetAll%20Enmy%20details) _array_index)))
            (Class|MineEnemy|MyReset _returnvalue))
          (goto _label Reset))))
    (:then_1
      ;[1 1 1] Resets objectives
      (Utilities|FlowControl|DoOnce false :!label _label_2
        (:Completed
          (bind _outactors_2 (Actor|GetAllActorsOfClass "/Game/Blueprints/Objectives/BP_UpdatedObjectivePoint.BP_UpdatedObjectivePoint_C"))
          (for _array_element_3 _outactors_2
            (Actor|DestroyActor _array_element_3))
          (for (_array_element_4 _array_index_2) (Variables|Default|GetLevelObjectives)
            (Game|SpawnActorfromClass (Utilities|GetClass _array_element_4) (Utilities|Array|Get(acopy) (Variables|Default|GetObjectiveTransforms) _array_index_2) "Undefined" "MultiplyWithRoot" 0 0))
          (goto _label_2 Reset))))
    (:then_2
      ;[1 1 1] Resets ship
      (Utilities|FlowControl|DoOnce false :!label _label_3
        (:Completed
          (bind _outactors_3 (Actor|GetAllActorsOfClass "/Game/Blueprints/Objectives/BP_UpdatedShipObjective.BP_UpdatedShipObjective_C"))
          (for _array_element_5 _outactors_3
            (Actor|DestroyActor))
          (for (_array_element_6 _array_index_3) (Variables|Default|GetShipObjectives)
            (Game|SpawnActorfromClass (Utilities|GetClass _array_element_6) (Utilities|Array|Get(acopy) (Variables|Default|GetShipObjectiveTransforms) _array_index_3) "Undefined" "MultiplyWithRoot" 0 0))
          (goto _label_3 Reset))))
    (:then_3
      ;[1 1 1] Reset Player game won
      (bind _returnvalue_2 (Actor|GetActorOfClass "/Game/Blueprints/Character/CharacterPresets/BP_PlayerCharPreset1.BP_PlayerCharPreset1_C"))
      (if (Variables|/Script/BladeBot.PlayerCharacter|GetGameComplete _returnvalue_2)
        (Variables|/Script/BladeBot.PlayerCharacter|SetGameComplete _returnvalue_2 false)))))