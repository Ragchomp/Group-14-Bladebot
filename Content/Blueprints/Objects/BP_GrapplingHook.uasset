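; BP_GrapplingHook is a grappling hook projectile that launches from its spawn point along the bladebot player's camera direction.
; On BeginPlay it caches the player, derives direction from a debug-drawn visibility trace's start and end, then impulses its physics-simulated box.
; If the Hit flag is false at launch, it destroys itself after a HookRange delay.
; The box's hit event leads to an empty sequence, so no latch or pull logic exists here.
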(event OnComponentHit(Box)
  (params (HitComponent :type Primitive%20Component%20Object%20Reference) (OtherActor :type Actor%20Object%20Reference) (OtherComp :type Primitive%20Component%20Object%20Reference) (NormalImpulse :type Vector :default "0, 0, 0") (Hit :type Hit%20Result%20Structure%20%28by%20ref%29))
  (Utilities|FlowControl|Sequence))

(event EventBeginPlay
  (bind _box (Variables|Default|GetBox))
  (Utilities|FlowControl|Sequence
    (:then_0
      ;[1 1 1] Setup
      (bind _asbp_bladebot (Utilities|Casting|CastToBP_bladebot (Game|Player|GetPlayerPawn 0)))
      (Variables|Default|SetPlayerCharacter _asbp_bladebot))
    (:then_1
      ;[1 1 1] Calculate direction
      (bind _outhit (Collision|LineTraceByChannel (Transformation|GetActorLocation (Variables|Default|GetPlayerCharacter)) (+ (Transformation|GetActorLocation (Variables|Default|GetPlayerCharacter)) (* (Math|Vector|GetForwardVector (Variables|/Game/Blueprints/Character/BP_bladebot.BP_bladebot_C|GetCamera (Variables|Default|GetPlayerCharacter))) (Variables|Default|GetHookDirMultiplier))) "TraceTypeQuery1" false 0 "ForDuration"))
      (Variables|Default|SetHookDirection (Math|Vector|GetUnitDirection(Vector) (.TraceStart (Collision|BreakHitResult _outhit)) (.TraceEnd (Collision|BreakHitResult _outhit)))))
    (:then_2
      ;[1 1 1] Fire Hook
      (Physics|SetSimulatePhysics _box true)
      (Physics|AddImpulse _box (* (Variables|Default|GetHookDirection) (Variables|Default|GetHookSpeed)) "None" true))
    (:then_4
      ;[1 1 1] Destroy If Miss
      (if (not (Variables|Default|GetHit))
        (Utilities|FlowControl|Delay (Variables|Default|GetHookRange))
        (Actor|DestroyActor)))))

(event Collision|EventActorBeginOverlap
  (params (OtherActor :type Actor%20Object%20Reference)))

(event EventTick
  (params (DeltaSeconds :type Float%20%28single-precision%29)))

(fn ConstructionScript)