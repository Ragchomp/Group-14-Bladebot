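; Player character Blueprint that drives a speed-lines effect from the character's movement speed.
; Each Tick maps PlayerMovementComponent velocity magnitude to a clamped spawn rate, sent to the Speedlines effect's Spawnrate variable, or zero at or below a cutoff.
; The key 1 DoOnce has nothing after it.
; A settings-screen toggle with cursor and input-mode switching, and a debug speed print, are disconnected and never run.
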(event EventBeginPlay)

(event Collision|EventActorBeginOverlap
  (params (OtherActor :type Actor%20Object%20Reference)))

(event EventTick
  (params (DeltaSeconds :type Float%20%28single-precision%29))
  (bind _playermovementcomponent (Variables|Default|GetPlayerMovementComponent))
  (bind _speedlines (Variables|Default|GetSpeedlines))
  (bind _velocity (Variables|/Script/Engine.MovementComponent|GetVelocity _playermovementcomponent))
  (bind _returnvalue (Math|Vector|VectorLength _velocity))
  (bind _returnvalue_2 (Math|Float|MapRangeClamped _returnvalue 0.0 8e+03 0.0 8e+01))
  (if (> _returnvalue_2 3e+01)
    (Niagara|SetNiagaraVariable(Float) _speedlines "Spawnrate" _returnvalue_2)
    (else
      (Niagara|SetNiagaraVariable(Float) _speedlines "Spawnrate" 0.0))))

(event Input|KeyboardEvents|1
  (params (Key :type Key%20Structure :default "None"))
  (:Pressed
    (Utilities|FlowControl|DoOnce false :!label _label))
  (:Released
    (goto _label Reset)))

(fn ConstructionScript)