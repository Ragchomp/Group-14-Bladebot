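; Easter egg enemy variant that inherits its damage response from a parent enemy class.
; On BeginPlay it registers its W component with the damage collision's attached joints.
; Death ragdolls Mesh and W, then, if an AI controller exists, unpossesses it and destroys the actor after a short delay.
; TriggerAttack is empty; leftover muzzle flash, sting effect and hit damage logic is disconnected and never runs.
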(event EventBeginPlay
  (|CallParentFunction)
  (Utilities|Array|AddUnique (Variables|/Game/Blueprints/Enemies/PlaceholderMehdi/EnemyLogic/EnemyDamageCollision.EnemyDamageCollision_C|GetAttatchedJoints (Variables|Default|GetEnemyDamageCollision1)) (Variables|Default|Getw)))

(event Collision|EventActorBeginOverlap
  (params (OtherActor :type Actor%20Object%20Reference))
  (|CallParentFunction OtherActor) ; This node is disabled and will not be called.\nDrag off pins to build functionality.
)

(event EventTick
  (params (DeltaSeconds :type Float%20%28single-precision%29)))

(event EventDamageResponse
  (params (Health :type Float%20%28double-precision%29))
  ;[1 1 1] Combat
  (|CallParentFunction Health))

(event EventTriggerAttack
  (params (Trace :type Hit%20Result%20Structure) (ShotCount :type Integer))
  ;[1 1 1] attack
)

(event EventDeath
  (bind _self self)
  (bind _returnvalue (AI|GetAIController _self))
  ;[1 1 1] Combat
  (|CallParentFunction)
  (Physics|SetSimulatePhysics (Variables|Character|GetMesh) true)
  (Physics|SetSimulatePhysics (Variables|Default|Getw) true)
  (Utilities|IsValid _returnvalue
    (:Is%20Valid
      (Pawn|UnPossess _returnvalue)
      (Utilities|FlowControl|Delay 2.0)
      (Actor|DestroyActor))))

(fn ConstructionScript
  (|CallParentFunction))