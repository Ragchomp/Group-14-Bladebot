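; Game instance for BladeBot that holds persistent game logic: player respawn, time-based scoring, and save/load.
; GetRefrence caches the player and game mode, whose timer feeds the score formula.
; RespawnPlayer revives a dead player at the stored location, or otherwise records the passed transform as that location.
; Save and load handle position, health and level through BP_SaveGame, with loading screens and delays covering level changes and state restoration.
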(event Custom|ScoreSystem
  (bind _game_mode (Variables|Default|GetGame%20Mode))
  (Variables|Default|SetScore 0)
  (Variables|Default|SetScore (+ (- 10000 (* (- (+ (Variables|/Game/Blueprints/Game/BP_BladeBotBaseGameMode.BP_BladeBotBaseGameMode_C|GetSeconds _game_mode) (* (Variables|/Game/Blueprints/Game/BP_BladeBotBaseGameMode.BP_BladeBotBaseGameMode_C|GetMinutes _game_mode) 60)) (Variables|Default|GetLevelMinTime)) (Variables|Default|GetTimeToScore))) (Variables|Default|GetScore))))

(event Custom|LoadGame
  (bind _playercharacter (Variables|Default|GetPlayerCharacter))
  ;[1 1 1] Load the game
  (bind _returnvalue (SaveGame|DoesSaveGameExist "savegame"))
  (if _returnvalue
    (bind _returnvalue_2 (SaveGame|LoadGamefromSlot (Variables|Default|GetSave%20Slot%20Name)))
    (bind _asbp_save_game (Utilities|Casting|CastToBP_SaveGame _returnvalue_2))
    (Variables|Default|SetSave%20Game _asbp_save_game)
    (else
      (bind _returnvalue_3 (SaveGame|CreateSaveGameObject "/Game/Blueprints/Game/BP_SaveGame.BP_SaveGame_C"))
      (Variables|Default|SetSave%20Game _returnvalue_3)))
  (Utilities|FlowControl|Sequence
    (:then_0
      (bind _returnvalue_4 (UserInterface|CreateWidget "/Game/Blueprints/Widget/WBP_LoadingScreen.WBP_LoadingScreen_C"))
      (bind _output_get (Variables|Default|SetLoadingScreen _returnvalue_4))
      (UserInterface|Viewport|AddtoViewport _output_get 0)
      (Input|SetInputModeUIOnly (Game|GetPlayerController 0) _output_get "DoNotLock" true))
    (:then_1
      (bind _returnvalue_5 (Game|GetCurrentLevelName true))
      (if (Utilities|Enum|Equal(Enum) _returnvalue_5 (Variables|/Game/Blueprints/Game/BP_SaveGame.BP_SaveGame_C|GetCurrentLevel (Variables|Default|GetSave%20Game)))
        _
        (else
          (Game|OpenLevel(byName) (Utilities|String|StringToName (Variables|/Game/Blueprints/Game/BP_SaveGame.BP_SaveGame_C|GetCurrentLevel (Variables|Default|GetSave%20Game))))
          (Utilities|FlowControl|Delay (Variables|Default|GetLoadingScreenDelay))
          (bind _returnvalue_6 (UserInterface|CreateWidget "/Game/Blueprints/Widget/WBP_LoadingScreen.WBP_LoadingScreen_C"))
          (bind _output_get_2 (Variables|Default|SetLoadingScreen2 _returnvalue_6))
          (UserInterface|Viewport|AddtoViewport _output_get_2 0)))
      (Transformation|SetActorLocation (Game|GetPlayerCharacter 0) (Variables|/Game/Blueprints/Game/BP_SaveGame.BP_SaveGame_C|GetPlayerPosition (Variables|Default|GetSave%20Game)) false false))
    (:then_2
      (Utilities|FlowControl|Delay (Variables|Default|GetLoadingScreenDelay))
      (Variables|/Game/Blueprints/Character/BP_bladebot.BP_bladebot_C|SetHealthCurrent _playercharacter (Variables|/Game/Blueprints/Game/BP_SaveGame.BP_SaveGame_C|GetHealth (Variables|Default|GetSave%20Game)))
      (Variables|/Game/Blueprints/Character/BP_bladebot.BP_bladebot_C|SetDeathCurrent _playercharacter false)
      (Default|UpdatePlayerStatus _playercharacter)
      (Variables|/Script/Engine.MovementComponent|SetVelocity (Pawn|GetMovementComponent _playercharacter) "0, 0, 0"))
    (:then_3
      (Utilities|FlowControl|Delay (Variables|Default|GetLoadingScreenDelay))
      (bind _loadingscreen (Variables|Default|GetLoadingScreen)
        (:then
          (Widget|RemovefromParent _loadingscreen))
        (:else
          _))
      (bind _loadingscreen2 (Variables|Default|GetLoadingScreen2)
        (:then
          (Widget|RemovefromParent _loadingscreen2))
        (:else
          _))
      (Input|SetInputModeGameOnly (Game|GetPlayerController 0) false))))

(event Custom|RespawnPlayer
  (params (InTransform :type Transform%20%28by%20ref%29))
  (bind _playercharacter (Variables|Default|GetPlayerCharacter))
  ;[1 1 1] Respawn Player character
  (if (Variables|/Game/Blueprints/Character/BP_bladebot.BP_bladebot_C|GetDeathCurrent (Variables|Default|GetPlayerCharacter))
    (Transformation|SetActorTransform (Variables|Default|GetPlayerCharacter) (Math|Transform|MakeTransform (.Location (Math|Transform|BreakTransform (Variables|Default|GetPlayerRespawnLocation)))) false true)
    (Variables|/Game/Blueprints/Character/BP_bladebot.BP_bladebot_C|SetDeathCurrent _playercharacter false)
    (Variables|/Game/Blueprints/Character/BP_bladebot.BP_bladebot_C|SetHealthCurrent _playercharacter 1e+02)
    (Variables|/Game/Blueprints/Character/BP_bladebot.BP_bladebot_C|SetIsLodged _playercharacter false)
    (Default|Clearhook _playercharacter)
    (Default|UpdatePlayerStatus _playercharacter)
    (else
      (Variables|Default|SetPlayerRespawnLocation InTransform))))

(event Custom|SaveGame
  ;[1 1 1] Save the Game
  (Utilities|IsValid (Variables|Default|GetSave%20Game)
    (:Is%20Valid
      _)
    (:Is%20Not%20Valid
      (bind _returnvalue (SaveGame|CreateSaveGameObject "/Game/Blueprints/Game/BP_SaveGame.BP_SaveGame_C"))
      (bind _output_get (Variables|Default|SetSave%20Game _returnvalue))))
  (Utilities|FlowControl|Sequence
    (:then_0
      (Variables|/Game/Blueprints/Game/BP_SaveGame.BP_SaveGame_C|SetPlayerPosition (Variables|Default|GetSave%20Game) (Transformation|GetActorLocation (Game|GetPlayerCharacter 0))))
    (:then_1
      (Variables|/Game/Blueprints/Game/BP_SaveGame.BP_SaveGame_C|SetHealth _output_get (.health (Variables|Default|GetPlayerStatus))))
    (:then_2
      (bind _returnvalue_2 (Game|GetCurrentLevelName true))
      (Variables|/Game/Blueprints/Game/BP_SaveGame.BP_SaveGame_C|SetCurrentLevel (Variables|Default|GetSave%20Game) _returnvalue_2)
      (SaveGame|SaveGametoSlot (Variables|Default|GetSave%20Game) (Variables|Default|GetSave%20Slot%20Name)))))

(event Custom|GetRefrence
  ;[1 1 1] Get reffrences
  (bind _asbp_bladebot (Utilities|Casting|CastToBP_bladebot (Game|GetPlayerCharacter 0)))
  (Variables|Default|SetPlayerCharacter _asbp_bladebot)
  (bind _asbp_blade_bot_base_game_mode (Utilities|Casting|CastToBP_BladeBotBaseGameMode (Game|GetGameMode)))
  (Variables|Default|SetGame%20Mode _asbp_blade_bot_base_game_mode))