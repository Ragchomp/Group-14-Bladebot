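; AI controller for a placeholder enemy that runs BT_EnemyPlaceholder on possession and manages aggro on the player.
; Perception updates on Player-tagged actors set the Target and HasLineOfSight blackboard keys.
; Losing sight clears line of sight at once but starts a short grace timer before dropping the target.
; Gaining or losing aggro also notifies BP_bladebot, the player character, to update its music state.
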(event OnTargetPerceptionUpdated(AIPerception)
  (params (Actor :type Actor%20Object%20Reference) (Stimulus :type AI%20Stimulus%20Structure))
  ;[1 1 1] Aggro
  (Variables|Default|SetPercieved%20actor Actor)
  (if (Actor|ActorHasTag Actor "Player")
    (if (.bSuccessfullySensed (Utilities|Struct|BreakAIStimulus Stimulus))
      (Utilities|Time|ClearandInvalidateTimerbyHandle (Variables|Default|GetLostSightTimer))
      (CallFunction|UpdateSight true)
      (CallFunction|UpdateTarget (Variables|Default|GetPercieved%20actor))
      (Default|MusicUpdateState (Variables|Default|GetPlayer) self true)
      (else
        (bind _returnvalue (Utilities|Time|SetTimerbyEvent (delegate Custom|AggroLoss) 5.0))
        (Variables|Default|SetLostSightTimer _returnvalue)
        (CallFunction|UpdateSight false)))))

(event Custom|AggroLoss
  ;[1 1 1] Aggro
  (CallFunction|UpdateTarget)
  (Default|MusicUpdateState (Variables|Default|GetPlayer) self false))

(event EventBeginPlay
  ;[1 1 1] Initial Setup
  (Utilities|FlowControl|Sequence
    (:then_0
      (bind _asbp_bladebot (Utilities|Casting|CastToBP_bladebot (Game|GetPlayerCharacter 0)))
      (Variables|Default|SetPlayer _asbp_bladebot))))

(event EventPossess
  (params (PossessedPawn :type Pawn%20Object%20Reference))
  (AI|RunBehaviorTree "/Game/Blueprints/Enemies/PlaceholderMehdi/EnemyLogic/BT_EnemyPlaceholder.BT_EnemyPlaceholder"))

(fn ConstructionScript)

(fn UpdateTarget
  (params (Target :type Actor%20Object%20Reference))
  (AI|Components|Blackboard|SetValueasObject (AI|GetBlackboard 0) (Utilities|Name|MakeLiteralName "Target") Target))

(fn UpdateSight
  (params (Has%20Line%20Of%20Sight :type Boolean))
  (AI|Components|Blackboard|SetValueasBool (AI|GetBlackboard 0) (Utilities|Name|MakeLiteralName "HasLineOfSight") Has%20Line%20Of%20Sight))