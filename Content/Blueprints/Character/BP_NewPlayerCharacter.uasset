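; Player character Blueprint holding a test toggle for the WBP_SettingsScreenTest settings widget, which is currently not connected.
; Key 1 drives a DoOnce that resets on release but triggers nothing.
; An unreachable FlipFlop alternates between creating the widget with a mouse cursor and Game-and-UI input, and removing it to restore game-only input.
; BeginPlay, Tick, overlap and the construction script are empty.
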(event EventBeginPlay)

(event Collision|EventActorBeginOverlap
  (params (OtherActor :type Actor%20Object%20Reference)))

(event EventTick
  (params (DeltaSeconds :type Float%20%28single-precision%29)))

(event Input|KeyboardEvents|1
  (params (Key :type Key%20Structure :default "None"))
  (:Pressed
    (Utilities|FlowControl|DoOnce false :!label _label))
  (:Released
    (goto _label Reset)))

(fn ConstructionScript)