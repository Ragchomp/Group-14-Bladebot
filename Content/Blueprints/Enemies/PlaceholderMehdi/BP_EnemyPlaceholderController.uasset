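; AI controller for the placeholder enemy that runs its behavior tree when it possesses a pawn.
; On BeginPlay it casts the player character to BP_bladebot and writes it to the blackboard's Player key.
; A call to update the player's music state exists in the graph but is unconnected and never runs.
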(event EventBeginPlay
  ;[1 1 1] Initial Setup
  (Utilities|FlowControl|Sequence
    (:then_0
      (bind _asbp_bladebot (Utilities|Casting|CastToBP_bladebot (Game|GetPlayerCharacter 0)))
      (Variables|Default|SetPlayer _asbp_bladebot))
    (:then_1
      (AI|Components|Blackboard|SetValueasObject (AI|GetBlackboard 0) (Utilities|Name|MakeLiteralName "Player") (Variables|Default|GetPlayer)))))

(event EventPossess
  (params (PossessedPawn :type Pawn%20Object%20Reference))
  (AI|RunBehaviorTree "/Game/Blueprints/Enemies/PlaceholderMehdi/BT_EnemyPlaceholder.BT_EnemyPlaceholder"))

(fn ConstructionScript)