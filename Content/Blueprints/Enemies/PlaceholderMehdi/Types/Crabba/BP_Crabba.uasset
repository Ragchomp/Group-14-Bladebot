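; BP_Crabba is an enemy Blueprint that implements the effects and damage of a traced ranged attack.
; TriggerAttack activates one of four muzzle components chosen by the shot count, then spawns a Niagara impact at the trace hit point, oriented by the inverted normal.
; It also draws a smoke beam between trace start and impact, then sends a fixed damage message to the hit actor.
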(event EventBeginPlay
  (|CallParentFunction) ; This node is disabled and will not be called.\nDrag off pins to build functionality.
)

(event Collision|EventActorBeginOverlap
  (params (OtherActor :type Actor%20Object%20Reference))
  (|CallParentFunction OtherActor) ; This node is disabled and will not be called.\nDrag off pins to build functionality.
)

(event EventTick
  (params (DeltaSeconds :type Float%20%28single-precision%29)))

(event EventTriggerAttack
  (params (Trace :type Hit%20Result%20Structure) (ShotCount :type Integer))
  ;[1 1 1] Attack
  (Utilities|FlowControl|Sequence
    (:then_0
      (Components|Activation|SetActive (Utilities|Select :Index ShotCount :Option%200 (Variables|Default|GetMuzzle) :Option%201 (Variables|Default|GetMuzzle1) :Option%202 (Variables|Default|GetMuzzle2) :Option%203 (Variables|Default|GetMuzzle3)) true true))
    (:then_1
      (bind _returnvalue (Niagara|SpawnSystematLocation "/Game/Assets/VFX/Crabba/Shooting/NS_StingImpact.NS_StingImpact" (.impactpoint Trace)))
      (Effects|Components|ParticleSystem|SetVectorParameter _returnvalue "HitDir" (* (.impactnormal Trace) -1.0)))
    (:then_2
      (bind _returnvalue_2 (Niagara|SpawnSystematLocation "/Game/Assets/VFX/Crabba/Shooting/NS_StingSmokeBeam.NS_StingSmokeBeam" (Transformation|GetActorLocation)))
      (Effects|Components|ParticleSystem|SetVectorParameter _returnvalue_2 "bulletEndPoint" (.impactpoint Trace))
      (Effects|Components|ParticleSystem|SetVectorParameter _returnvalue_2 "bulletStartPoint" (.tracestart Trace)))
    (:then_3
      (Class|BPIDamage|Damage(Message) (.hitactor Trace) false 2e+01 1.0 "NewEnumerator0" "NewEnumerator0"))))

(fn ConstructionScript
  (|CallParentFunction))