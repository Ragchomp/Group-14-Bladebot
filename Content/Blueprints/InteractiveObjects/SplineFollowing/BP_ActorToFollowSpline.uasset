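; Actor that travels along a spline from start to end, picking a random BP_SplineForFollowing in the level on BeginPlay.
; A timeline, with play rate set to the inverse of TimeToComplete, drives a lerp over the spline's length.
; Each update sets the actor's world location and rotation to match the spline at that distance.
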(event Custom|Move%20object
  (bind _splineref (Variables|Default|GetSplineRef))
  (bind _spline (Variables|/Game/Blueprints/InteractiveObjects/SplineFollowing/BP_SplineForFollowing.BP_SplineForFollowing_C|GetSpline _splineref))
  ;[1 1 1] Move the actor along the spline with the given time verriable
  (Components|Timeline|SetPlayRate (Variables|Default|GetMoveObjectT) (/ 1.0 (Variables|Default|GetTimeToComplete)))
  (bind _movetrack (Timeline|MoveObjectT Play)
    (:Update
      (Transformation|SetActorTransform (Math|Transform|MakeTransform (Spline|GetLocationatDistanceAlongSpline _spline (Math|Float|Lerp 0.0 (Spline|GetSplineLength (Variables|/Game/Blueprints/InteractiveObjects/SplineFollowing/BP_SplineForFollowing.BP_SplineForFollowing_C|GetSpline (Variables|Default|GetSplineRef))) _movetrack) "World") (Spline|GetRotationatDistanceAlongSpline _spline (Math|Float|Lerp 0.0 (Spline|GetSplineLength (Variables|/Game/Blueprints/InteractiveObjects/SplineFollowing/BP_SplineForFollowing.BP_SplineForFollowing_C|GetSpline (Variables|Default|GetSplineRef))) _movetrack) "World") "1.000000,1.000000,1.000000")))))

(event EventBeginPlay
  ;[1 1 1] Set refrence of what spline to follow
  ;;[1 1 1] When creating a new object to follow a spline, set the spesific spline here.
  (bind _outactors (Actor|GetAllActorsOfClass "/Game/Blueprints/InteractiveObjects/SplineFollowing/BP_SplineForFollowing.BP_SplineForFollowing_C"))
  (Variables|Default|SetSplineRef (.OutItem (Utilities|Array|Random _outactors)))
  (CallFunction|MoveObject))

(fn ConstructionScript)