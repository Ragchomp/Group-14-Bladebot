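; Base game mode for BladeBot combat that sets up the HUD, minimap markers, and pause and options menus.
; BeginPlay adds the combat HUD, spawns an owned BP_Sprite on each "Enemy"-tagged actor for the minimap, and caches the movement controller.
; Pause swaps all widgets for the pause menu, or unpauses, restores game-only input and recreates the HUD.
; The options toggle remembers the calling widget class to recreate it on return.
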(event Custom|Pause
  (params (Condition :type Boolean))
  (bind _returnvalue (Game|GetPlayerController 0))
  ;[1 1 1] pause event
  (if Condition
    (Viewport|RemoveAllWidgets)
    (bind _returnvalue_2 (UserInterface|CreateWidget "/Game/Blueprints/Widget/WBP_PauseMenu.WBP_PauseMenu_C"))
    (bind _output_get (Variables|Default|SetPauseWiget _returnvalue_2))
    (UserInterface|Viewport|AddtoViewport _output_get 0)
    (else
      (Variables|/Game/Blueprints/Character/BP_BladebotMovementController.BP_BladebotMovementController_C|SetPaused (Variables|Default|GetPlayerController) false)
      (Game|SetGamePaused false)
      (Viewport|RemoveAllWidgets)
      (Variables|/Script/Engine.PlayerController|SetbShowMouseCursor _returnvalue false)
      (Input|SetInputModeGameOnly _returnvalue false)
      (bind _returnvalue_3 (UserInterface|CreateWidget "/Game/Blueprints/Widget/WBP_CombatHUD.WBP_CombatHUD_C"))
      (UserInterface|Viewport|AddtoViewport _returnvalue_3 0))))

(event Custom|RetrunFromOptionBot
  (params (Class :type User%20Widget%20Class%20Reference) (Target :type Widget%20Object%20Reference))
  ;[1 1 1] Open and close options
  (if (Variables|Default|GetInOptions)
    (Variables|Default|SetInOptions false)
    (bind _returnvalue (UserInterface|CreateWidget (Variables|Default|GetOptionWiget)))
    (Widget|RemovefromParent (stale _returnvalue_2))
    (UserInterface|Viewport|AddtoViewport _returnvalue 0)
    (else
      (Variables|Default|SetInOptions true)
      (Variables|Default|SetOptionWiget Class)
      (bind _returnvalue_2 (UserInterface|CreateWidget "/Game/Blueprints/Widget/WBP_OptionMenu.WBP_OptionMenu_C"))
      (Widget|RemovefromParent Target)
      (UserInterface|Viewport|AddtoViewport _returnvalue_2 0))))

(event EventBeginPlay
  (Utilities|FlowControl|Sequence
    (:then_0
      ;[1 1 1] Add hud for base combat
      (bind _returnvalue (UserInterface|CreateWidget "/Game/Blueprints/Widget/WBP_CombatHUD.WBP_CombatHUD_C"))
      (UserInterface|Viewport|AddtoViewport _returnvalue 0))
    (:then_1
      ;[1 1 1] Spawn sprite for minimap on all with tag
      (bind _outactors (Actor|GetAllActorswithTag "Enemy"))
      (for _array_element _outactors
        (Game|SpawnActorfromClass "/Game/Blueprints/Game/BP_Sprite.BP_Sprite_C" (Transformation|GetActorTransform _array_element) "Undefined" _array_element 0)))
    (:then_2
      (bind _asbp_bladebot_movement_controller (Utilities|Casting|CastToBP_BladebotMovementController (Game|GetPlayerController 0)))
      (Variables|Default|SetPlayerController _asbp_bladebot_movement_controller))))

(fn ConstructionScript)