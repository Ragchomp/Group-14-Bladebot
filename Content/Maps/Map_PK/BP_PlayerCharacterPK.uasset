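; Player character Blueprint for the PK map that adds two slow-motion controls through global time dilation, each with slow-down and speed-up sounds.
; Key 1 toggles the effect with a FlipFlop, playing or reversing a timeline that drives the dilation value.
; Key 2 triggers a timed burst on a second timeline, which reverses automatically after a short Delay that runs in dilated game time.
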(event EventBeginPlay)

(event Collision|EventActorBeginOverlap
  (params (OtherActor :type Actor%20Object%20Reference)))

(event Input|KeyboardEvents|1
  (params (Key :type Key%20Structure))
  ;[1 1 1] ToggleSlowdown
  (:Pressed
    (Utilities|FlowControl|FlipFlop
      (:A
        (Audio|PlaySound2D "/Game/Assets/Sound/Effects/SlowDown.SlowDown" 1.0 1.0 0.0 0 0)
        (bind _time_track (Timeline|Timeline Play)
          (:Update
            (Utilities|Time|SetGlobalTimeDilation _time_track))))
      (:B
        (Audio|PlaySound2D "/Game/Assets/Sound/Effects/SpeedUp.SpeedUp" 1.0 1.0 0.0 0 0)
        (Timeline|Timeline Reverse)))))

(event Input|KeyboardEvents|2
  (params (Key :type Key%20Structure))
  ;[1 1 1] DurationSlowdown
  (:Pressed
    (Utilities|FlowControl|Sequence
      (:then_0
        (Audio|PlaySound2D "/Game/Assets/Sound/Effects/SlowDown.SlowDown" 1.0 1.0 0.0 0 0)
        (bind _time_track (Timeline|Timeline_0 Play)
          (:Update
            (Utilities|Time|SetGlobalTimeDilation _time_track))))
      (:then_1
        (Utilities|FlowControl|Delay 0.6)
        (Audio|PlaySound2D "/Game/Assets/Sound/Effects/SpeedUp.SpeedUp" 1.0 1.0 0.0 0 0)
        (Timeline|Timeline_0 Reverse)))))

(fn ConstructionScript)