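; BP_bladebot is the player character, a blade robot that grapples with a hook, slides its tip through surfaces until it lodges, and damages what its blade overlaps while attacking.
; Tick drives state-based rotation (grappling, sliding, lodged, airborne), spark and speedline effects, music parameters and projectile-path prediction of hook hits.
; Incoming damage applies falloff and resistances, updates GameInstance status, and triggers respawn on death.
; BeginPlay caches references, attaches a minimap and shows a loading screen.
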(event Custom|HookHit
  ;[1 1 1] Successful Hook
  (Utilities|FlowControl|Sequence
    (:then_0
      (Variables|Physics|SetIsGrappling true))
    (:then_1
      (Variables|PostLanding|SetIsLodged false))
    (:then_2
      (Utilities|FlowControl|Sequence
        (:then_0
          (Physics|SetSimulatePhysics (Variables|Collision|GetCapsuleComponent) true))))))

(event Custom|Clearhook
  ;[1 1 1] Remove Hook
  (Utilities|FlowControl|Sequence
    (:then_0
      (Variables|Physics|SetIsGrappling false))
    (:then_1
      (Variables|Physics|SethasGrappled true))
    (:then_2
      (Utilities|FlowControl|Sequence
        (:then_0
          (Physics|SetSimulatePhysics (Variables|Collision|GetCapsuleComponent) false))
        (:then_1
          (Utilities|IsValid (Variables|/Game/Blueprints/Character/BP_BladebotMovementController.BP_BladebotMovementController_C|GetHookRef (Variables|Components|GetMovementController))
            (:Is%20Valid
              (Actor|DestroyActor (Variables|/Game/Blueprints/Character/BP_BladebotMovementController.BP_BladebotMovementController_C|GetHookRef (Variables|Components|GetMovementController))))))))))

(event Custom|UpdatePlayerStatus
  (Utilities|FlowControl|Sequence
    (:then_0
      ;[1 1 1] SetHealth
      (bind _output_get (Variables|/Game/Blueprints/Game/BP_BladeBotGameInstance.BP_BladeBotGameInstance_C|SetPlayerStatus (Variables|Components|GetGameInstance) (Utilities|Struct|MakeStruct_PlayerStatus (Variables|Status|GetHealthCurrent) (Variables|Status|GetDeathCurrent))))
      ;[1 1 1] Debughealth
      (Development|PrintString (Utilities|String|ToString(Float) (.Health (Utilities|Struct|BreakStruct_PlayerStatus _output_get))) true true "(R=1.000000,G=0.045011,B=0.000000,A=1.000000)" 2.0 "1")
      (Utilities|FlowControl|Sequence
        (:then_0
          ;[1 1 1] check if Health is less than 0
          (if (<= (.health (Variables|/Game/Blueprints/Game/BP_BladeBotGameInstance.BP_BladeBotGameInstance_C|GetPlayerStatus (Variables|Components|GetGameInstance))) 0.0)
            (CallFunction|Kill)))))))

(event Custom|Kill
  ;[1 1 1] Kills Player
  (Variables|Status|SetDeathCurrent true)
  (Variables|/Game/Blueprints/Game/BP_BladeBotGameInstance.BP_BladeBotGameInstance_C|SetPlayerStatus (Variables|Components|GetGameInstance) (Utilities|Struct|MakeStruct_PlayerStatus (Variables|Status|GetHealthCurrent) (Variables|Status|GetDeathCurrent)))
  (Default|RespawnPlayer (Variables|Components|GetGameInstance)))

(event EventBeginPlay
  ;[1 1 1] Initialize
  (Utilities|FlowControl|Sequence
    (:then_0
      (bind _asbp_bladebot_movement_controller (Utilities|Casting|CastToBP_BladebotMovementController (Game|GetPlayerController 0)))
      (Variables|Components|SetMovementController _asbp_bladebot_movement_controller))
    (:then_1
      (Variables|/Game/Blueprints/Character/BP_BladebotMovementController.BP_BladebotMovementController_C|SetDefaultCameraArmLength (Variables|Components|GetMovementController) (Variables|/Script/Engine.SpringArmComponent|GetTargetArmLength (Variables|Default|GetSpringArm)))
      (Variables|AnimationValues|SetCached%20Rotation (Transformation|GetActorRotation)))
    (:then_2
      (bind _asbp_blade_bot_game_instance (Utilities|Casting|CastToBP_BladeBotGameInstance (Game|GetGameInstance)))
      (bind _output_get (Variables|Components|SetGameInstance _asbp_blade_bot_game_instance))
      (Default|GetRefrence _output_get))
    (:then_3
      (|MinimapInitializer))
    (:then_4
      (bind _returnvalue (UserInterface|CreateWidget "/Game/Blueprints/Widget/WBP_LoadingScreen.WBP_LoadingScreen_C"))
      (UserInterface|Viewport|AddtoViewport _returnvalue 0)
      (Utilities|FlowControl|Delay 3.0)
      (Widget|RemovefromParent _returnvalue))))

(event EventTick
  (params (DeltaSeconds :type Float%20%28single-precision%29))
  ;[1 1 1] Tick Events
  (Utilities|FlowControl|Sequence
    (:then_0
      (|ActorTransform))
    (:then_1
      (|MusicUpdateGraph))
    (:then_2
      (|HookHitCheck))
    (:then_3
      (|AnimationValues))))

(event Input|KeyboardEvents|1
  (params (Key :type Key%20Structure :default "None"))
  (:Pressed
    (Default|SaveGame (Variables|Components|GetGameInstance))))

(event Input|KeyboardEvents|2
  (params (Key :type Key%20Structure :default "None"))
  (:Pressed
    (Default|LoadGame (Variables|Components|GetGameInstance))))

(fn ConstructionScript)

(event OnComponentBeginOverlap(Tip)
  (params (OverlappedComponent :type Primitive%20Component%20Object%20Reference) (OtherActor :type Actor%20Object%20Reference) (OtherComp :type Primitive%20Component%20Object%20Reference) (OtherBodyIndex :type Integer) (bFromSweep :type Boolean) (SweepResult :type Hit%20Result%20Structure%20%28by%20ref%29))
  (bind _returnvalue (Collision|GetCollisionObjectType OtherComp))
  ;[1 1 1] Check If Tip Is overlapping Ground Or wall
  (if (Variables|Physics|GethasGrappled)
    (if (not (Variables|PostLanding|GetIsLodged))
      (if (or (Utilities|Enum|Equal(Enum) _returnvalue "ECC_GameTraceChannel3") (Utilities|Enum|Equal(Enum) _returnvalue "ECC_GameTraceChannel4"))
        (Variables|PostLanding|SetSwordSliding true)
        (Variables|PostLanding|SetIsLodged false)
        (bind _returnvalue_2 (Niagara|SpawnSystematLocation "/Game/Assets/VFX/Player/Sparks/NS_Sparks.NS_Sparks" (Transformation|GetActorLocation)))
        (Variables|PostLanding|SetNSSparks _returnvalue_2)
        (else
          (Variables|PostLanding|SetSwordSliding false))))))

(event OnComponentBeginOverlap(Groundcheck)
  (params (OverlappedComponent :type Primitive%20Component%20Object%20Reference) (OtherActor :type Actor%20Object%20Reference) (OtherComp :type Primitive%20Component%20Object%20Reference) (OtherBodyIndex :type Integer) (bFromSweep :type Boolean) (SweepResult :type Hit%20Result%20Structure%20%28by%20ref%29))
  ;[1 1 1] Check is Body Is overlapping Ground
  (if (Variables|Physics|GethasGrappled)
    (if (Utilities|Enum|Equal(Enum) (Collision|GetCollisionObjectType OtherComp) "ECC_GameTraceChannel3")
      (Variables|PostLanding|SetIsContactingFloor true)
      (else
        (Variables|PostLanding|SetIsContactingFloor false :!label _label)))
    (else
      (goto _label))))

(event OnComponentBeginOverlap(Fullblade)
  (params (OverlappedComponent :type Primitive%20Component%20Object%20Reference) (OtherActor :type Actor%20Object%20Reference) (OtherComp :type Primitive%20Component%20Object%20Reference) (OtherBodyIndex :type Integer) (bFromSweep :type Boolean) (SweepResult :type Hit%20Result%20Structure%20%28by%20ref%29))
  (CallFunction|Attack OtherComp))

(event Custom|Attack
  (params (Target :type Object%20Object%20Reference))
  (if (Variables|Combat|GetIsAttacking)
    (Class|BPIDamage|Damage(Message) Target false 1e+01 1.0 "NewEnumerator0" "NewEnumerator0")))

(event Custom|MusicUpdateVariables
  (bind _returnvalue (Transformation|GetVelocity))
  (bind _returnvalue_2 (Math|Vector|VectorLength _returnvalue))
  ;[1 1 1] Floats
  (Utilities|FlowControl|Sequence
    (:then_0
      (if (> _returnvalue_2 2.3e+03)
        (Audio|Parameter|SetFloatParameter (Variables|Default|GetMusic) "FallingExponent" (Math|Float|MapRangeClamped _returnvalue_2 0.0 8e+03 0.0 0.5) :!class /Script/AudioExtensions.AudioParameterControllerInterface)
        (else
          (Audio|Parameter|SetFloatParameter (Variables|Default|GetMusic) "FallingExponent" 0.0 :!class /Script/AudioExtensions.AudioParameterControllerInterface))))))

(event Custom|MusicUpdateState
  (params (AggroedEnemy :type Actor%20Object%20Reference%20%28by%20ref%29) (AddedOrRemoved :type Boolean))
  ;[1 1 1] Combat
  (Utilities|FlowControl|Sequence
    (:then_0
      (if AddedOrRemoved
        (Utilities|Array|Add (Variables|Combat|GetEnemyAggroArray) AggroedEnemy)
        (else
          (Utilities|Array|RemoveItem (Variables|Combat|GetEnemyAggroArray) AggroedEnemy))))
    (:then_1
      (Effects|Components|ParticleSystem|SetBoolParameter (Variables|Default|GetMusic) "Combat" (Utilities|Array|IsNotEmpty (Variables|Combat|GetEnemyAggroArray))))))

(event EventDamage
  (params (UnmitigatedDamage :type Boolean) (DamageAmount :type Float%20%28double-precision%29) (DistanceFalloff :type Float%20%28double-precision%29) (DamageTypePrimary :type Enum_PrimaryDamageTypes%20Enum :default "NewEnumerator0") (DamageTypeSecondary :type Enum_SecondaryDamagetypes%20Enum :default "NewEnumerator0"))
  (bind _gameinstance (Variables|Components|GetGameInstance))
  (bind _playerstats (Variables|/Game/Blueprints/Game/BP_BladeBotGameInstance.BP_BladeBotGameInstance_C|GetPlayerStats _gameinstance))
  (Utilities|FlowControl|Sequence
    (:then_0
      (Variables|Damage|SetPremitigatedDamage DamageAmount))
    (:then_1
      (Variables|Damage|SetDistanceFalloffMultiplier DistanceFalloff))
    (:then_2
      (Variables|Physics|SetUnmitigated%20Damage UnmitigatedDamage))
    (:then_3
      (Variables|Damage|SetDamageAfterFalloff (* (Variables|Damage|GetPremitigatedDamage) (Variables|Damage|GetDistanceFalloffMultiplier)))
      (Variables|Damage|SetDamageAfterPrimaryType (Utilities|Select :Index DamageTypePrimary :NewEnumerator0 (Math|Float|Clamp(Float) (- (Variables|Damage|GetDamageAfterFalloff) (.rangedresist _playerstats)) 1.0 99999.0) :NewEnumerator1 (Math|Float|Clamp(Float) (- (Variables|Damage|GetDamageAfterFalloff) (.meleeresist _playerstats)) 1.0 99999.0)))
      (Variables|Damage|SetDamageAfterSecondaryType (Utilities|Select :Index DamageTypeSecondary :NewEnumerator0 (Math|Float|Clamp(Float) (- (Variables|Damage|GetDamageAfterPrimaryType) (.physicalresist _playerstats)) 1.0 99999.0) :NewEnumerator1 (Math|Float|Clamp(Float) (- (Variables|Damage|GetDamageAfterPrimaryType) (.energyresist _playerstats)) 1.0 99999.0)))
      ;[1 1 1] Use Resistances
      (if (Variables|Physics|GetUnmitigated%20Damage)
        ;[1 1 1] Resolve
        (Variables|Status|SetHealthCurrent (- (.health (Variables|/Game/Blueprints/Game/BP_BladeBotGameInstance.BP_BladeBotGameInstance_C|GetPlayerStatus (Variables|Components|GetGameInstance))) (Variables|Damage|GetDamageAfterFalloff)))
        (else
          (Variables|Status|SetHealthCurrent (- (.health (Variables|/Game/Blueprints/Game/BP_BladeBotGameInstance.BP_BladeBotGameInstance_C|GetPlayerStatus (Variables|Components|GetGameInstance))) (Variables|Damage|GetDamageAfterSecondaryType)))))
      (CallFunction|UpdatePlayerStatus))))