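; BP_MasterFadeActor is an actor that fades its static mesh in and out through a material parameter.
; The construction script creates a dynamic instance of each mesh material, stores them in an array and assigns them back to the material slots by index.
; Fadein plays a timeline that writes its value to the "Fade" scalar parameter on every instance, and FadeOut reverses that timeline.
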(event EventBeginPlay)

(event Collision|EventActorBeginOverlap
  (params (OtherActor :type Actor%20Object%20Reference)))

(event EventTick
  (params (DeltaSeconds :type Float%20%28single-precision%29)))

(event EventFadein
  (bind _fade (Timeline|Timeline Play)
    (:Update
      (for _array_element (Variables|Default|GetDynamic%20Material%20Instances)
        (Rendering|Material|SetScalarParameterValue _array_element "Fade" _fade :!class /Script/Engine.MaterialInstanceDynamic)))))

(event EventFadeOut
  (bind _fade (Timeline|Timeline Reverse)
    (:Update
      (for _array_element (Variables|Default|GetDynamic%20Material%20Instances)
        (Rendering|Material|SetScalarParameterValue _array_element "Fade" _fade :!class /Script/Engine.MaterialInstanceDynamic)))))

(fn ConstructionScript
  (Utilities|Array|Clear (Variables|Default|GetDynamic%20Material%20Instances))
  (for _array_element (Rendering|Material|GetMaterials (Variables|Default|GetStaticMesh))
    (bind _returnvalue (Rendering|Material|CreateDynamicMaterialInstance _array_element "None" "None" :!class /Script/Engine.KismetMaterialLibrary))
    (Utilities|Array|AddUnique (Variables|Default|GetDynamic%20Material%20Instances) _returnvalue)
    (CallFunction|SetMaterialstoDynamicInstances)))

(fn SetMaterialstoDynamicInstances
  (for (_array_element _array_index) (Variables|Default|GetDynamic%20Material%20Instances)
    (Rendering|Material|SetMaterial (Variables|Default|GetStaticMesh) _array_index _array_element)))